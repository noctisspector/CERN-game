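; Player character Blueprint that handles movement and look input, with a head bob camera shake while moving.
; Vertical and horizontal move axes feed scaled forward and right vectors into the CharacterMovement component, while look axes drive controller pitch and yaw.
; Both move events share a velocity check that plays the HeadBob_BP world camera shake at the actor's location whenever velocity is non-zero.
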(event `InputAxis|Move Vertical`
  (params (AxisValue :type "Float (single-precision)"))
  ;[1 1 1] Movement
  (`PawnMovementComponent.AddInputVector` (`self.CharacterMovement`) (* (`self.GetActorForwardVector`) AxisValue) false)
  ;[1 1 1] Movement Shake
  (if (not (== (`KismetMathLibrary.VSizeSquared` (`self.GetVelocity`)) 0.0)) :!label _label
    (`GameplayStatics.PlayWorldCameraShake` "/Game/Blueprint/Shake/HeadBob_BP.HeadBob_BP_C" (`self.K2_GetActorLocation`) 400.0 400.0)))

(event `InputAxis|Move Horizontal`
  (params (AxisValue :type "Float (single-precision)"))
  ;[1 1 1] Movement
  (`PawnMovementComponent.AddInputVector` (`self.CharacterMovement`) (* (`self.GetActorRightVector`) AxisValue) false)
  (goto _label))

(event `InputAxis|Look Vertical`
  (params (AxisValue :type "Float (single-precision)"))
  ;[1 1 1] Look
  (`self.AddControllerPitchInput` AxisValue))

(event `InputAxis|Look Horizontal`
  (params (AxisValue :type "Float (single-precision)"))
  ;[1 1 1] Look
  (`self.AddControllerYawInput` AxisValue))

(fn `UserConstructionScript`)