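; Geiger counter actor that reads radiation from every RadSource_BP in the level and shows it on a needle meter.
; Each tick it sums source strength with inverse-square distance falloff, clamped to min and max limits.
; That total sets the chance of random clicks, each playing a sound and bumping a reading that decays proportionally over time.
; The reading rotates the poseable mesh's Meter bone to move the needle.
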(event `self.ReceiveBeginPlay`
  (bind _outactors (`GameplayStatics.GetAllActorsOfClass` "/Game/Blueprint/Env/RadSource_BP.RadSource_BP_C"))
  (set `self.Sources` _outactors))

(event `self.ReceiveTick`
  (params (DeltaSeconds :type "Float (single-precision)"))
  (bind _current_reading (`self.Current Reading`))
  (`|ExecutionSequence`
    (:`then_0`
      ;[1 1 1] Find Total Radiation Strength
      (set `self.Total Strength` 0.0)
      (for _array_element (`self.Sources`)
        (set `self.Total Strength` (`KismetMathLibrary.FClamp` (+ (/ (`/Game/Blueprint/Env/RadSource_BP.Strength` _array_element) (`KismetMathLibrary.Square` (* (`KismetMathLibrary.FClamp` (`self.GetDistanceTo` _array_element) (`/Game/Blueprint/Env/RadSource_BP.Source Radius` _array_element) 50000.0) (`self.World Strength`)))) (`self.Total Strength`)) (`self.Min Strength`) (`self.Max Strength`)))))
    (:`then_1`
      ;[1 1 1] Decrease Reading
      (set `self.Current Reading` (`KismetMathLibrary.FClamp` (- _current_reading (* DeltaSeconds _current_reading (`self.Current Fallback Speed`))) 0.0 1000.0))
      ;[1 1 1] Random Readings
      (if (< (- (/ 1.0 (`KismetMathLibrary.RandomFloat`)) 1.0) (`self.Total Strength`))
        (set `self.Current Reading` (+ (`self.Current Reading`) (`self.Reading Strength`)))
        (`GameplayStatics.PlaySound2D` "/Engine/VREditor/Sounds/VR_click2.VR_click2" 0.05 1.0 0.0 null null)))
    (:`then_2`
      ;[1 1 1] Adjust Mesh Meter
      (`PoseableMeshComponent.SetBoneRotationByName` (`self.PoseableMesh`) "Meter" (`KismetMathLibrary.MakeRotator` 0.0 0.0 (`KismetMathLibrary.MapRangeClamped` (`self.Current Reading`) 0.0 50.0 -32.0 36.0)) "ComponentSpace"))))

(fn `UserConstructionScript`
  (`parent.UserConstructionScript`))